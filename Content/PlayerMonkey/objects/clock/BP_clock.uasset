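; BP_clock is a clock pickup that adds six seconds to the BP_monk timer when overlapped.
; A short delay after BeginPlay arms the Cooldown flag that gates overlaps.
; On pickup it rolls seconds above sixty into minutes, destroys itself and plays the banana collect sound.
; The mesh is destroyed before the cast, so any overlapping actor removes it, and the Tick rotation is zero.
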(event `self.ReceiveBeginPlay`
  (`KismetSystemLibrary.Delay` 0.5)
  (set `self.Cooldown` true))

(event `self.ReceiveTick`
  (params (DeltaSeconds :type "Float (single-precision)"))
  (`SceneComponent.K2_AddRelativeRotation` :`self` (`self.StaticMesh`)))

(event `self.ReceiveActorBeginOverlap`
  (params (OtherActor :type "Actor Object Reference"))
  (if (`self.Cooldown`)
    (`ActorComponent.K2_DestroyComponent` (`self.StaticMesh`))
    (bind _asbp_monk (cast `/Game/PlayerMonkey/player/BP_monk` OtherActor))
    (bind _output_get (set `/Game/PlayerMonkey/player/BP_monk.Seconds` (+ (`/Game/PlayerMonkey/player/BP_monk.Seconds` _asbp_monk) 6) _asbp_monk))
    (if (> _output_get 60)
      (set `/Game/PlayerMonkey/player/BP_monk.Seconds` (- (`/Game/PlayerMonkey/player/BP_monk.Seconds` _asbp_monk) 60) _asbp_monk)
      (set `/Game/PlayerMonkey/player/BP_monk.Minutes` (+ (`/Game/PlayerMonkey/player/BP_monk.Minutes` _asbp_monk) 1) _asbp_monk)
      (`self.K2_DestroyActor`)
      (`GameplayStatics.PlaySound2D` "/Game/PlayerMonkey/audio___musics/collect_the_banana.collect_the_banana" 2.5 1.0 0.0 null null)
      (else
        (`self.K2_DestroyActor`)
        (`GameplayStatics.PlaySound2D` "/Game/PlayerMonkey/audio___musics/collect_the_banana.collect_the_banana" 2.5 1.0 0.0 null null)))))

(fn `UserConstructionScript`)